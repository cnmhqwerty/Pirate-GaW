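; MapPieceChest_BP is an interactable chest that gives the player a map piece.
; Box overlap with the top-down character toggles input and a gate, so Interact only works in range.
; Interacting increments the character's MapCount, shows a GetMap widget for one second, plays a sound, then destroys the chest.
; A second Interact handler only casts the game mode and does nothing further.
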(event `InputAction|Interact`
  (params (Key :type "Key Structure"))
  (:`Pressed`
    (cast `/Game/TopDown/Blueprints/BP_TopDownGameMode` (`GameplayStatics.GetGameMode`))))

(event `InputAction|Interact`
  (params (Key :type "Key Structure"))
  (:`Pressed`
    (`/Engine/EditorBlueprintResources/StandardMacros.Gate` true :!label _label
      (:`Exit`
        (bind _asbp_top_down_character (cast `/Game/TopDown/Blueprints/BP_TopDownCharacter` (`GameplayStatics.GetPlayerCharacter` 0)))
        (set `/Game/TopDown/Blueprints/BP_TopDownCharacter.MapCount` (+ (`/Game/TopDown/Blueprints/BP_TopDownCharacter.MapCount` _asbp_top_down_character) 1) _asbp_top_down_character)
        (bind _returnvalue (`|CreateWidget` "/Game/Blueprints/GetMap.GetMap_C"))
        (`UserWidget.AddToPlayerScreen` _returnvalue 0)
        (`KismetSystemLibrary.Delay` 1.0)
        (`Widget.RemoveFromParent` _returnvalue)
        (`GameplayStatics.PlaySound2D` "/Engine/VREditor/Sounds/UI/Foliage_Placed.Foliage_Placed" 1.0 1.0 0.0 null null)
        (`self.K2_DestroyActor`)))))

(event `self.Box.OnComponentBeginOverlap`
  (params (OverlappedComponent :type "PrimitiveComponent Object Reference") (OtherActor :type "Actor Object Reference") (OtherComp :type "PrimitiveComponent Object Reference") (OtherBodyIndex :type Integer) (bFromSweep :type Boolean) (SweepResult :type "HitResult Structure (by ref)"))
  (cast `/Game/TopDown/Blueprints/BP_TopDownCharacter` OtherActor)
  (`self.EnableInput` (`GameplayStatics.GetPlayerController` 0))
  (goto _label :!via `Open`))

(event `self.Box.OnComponentEndOverlap`
  (params (OverlappedComponent :type "PrimitiveComponent Object Reference") (OtherActor :type "Actor Object Reference") (OtherComp :type "PrimitiveComponent Object Reference") (OtherBodyIndex :type Integer))
  (cast `/Game/TopDown/Blueprints/BP_TopDownCharacter` OtherActor)
  (`self.DisableInput` (`GameplayStatics.GetPlayerController` 0))
  (goto _label :!via `Close`))

(fn `UserConstructionScript`)