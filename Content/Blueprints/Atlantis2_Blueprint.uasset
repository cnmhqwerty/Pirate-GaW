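; Atlantis2 actor that acts as the win objective, unlocked once the overlapping BP_TopDownCharacter has a MapCount of at least 9.
; Overlapping Box enables that character's input and plays the RaiseTrack timeline, lerping the static mesh from the Start to the End relative location.
; Overlapping Win with the same count shows WinWidget and the mouse cursor, pauses the game and destroys the actor.
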(event `self.Box.OnComponentBeginOverlap`
  (params (OverlappedComponent :type "PrimitiveComponent Object Reference") (OtherActor :type "Actor Object Reference") (OtherComp :type "PrimitiveComponent Object Reference") (OtherBodyIndex :type Integer) (bFromSweep :type Boolean) (SweepResult :type "HitResult Structure (by ref)"))
  (bind _asbp_top_down_character (cast `/Game/TopDown/Blueprints/BP_TopDownCharacter` OtherActor))
  (`/Engine/EditorBlueprintResources/StandardMacros.CompareInt` (`/Game/TopDown/Blueprints/BP_TopDownCharacter.MapCount` _asbp_top_down_character) 9
    (:`>`
      _)
    (:`==`
      _))
  (`self.EnableInput` OtherActor (`GameplayStatics.GetPlayerController` 0))
  (bind (_direction _raise) (`Timeline|RaiseTrack` :`NewTime` 2.0)
    (:`Update`
      (`SceneComponent.K2_SetRelativeLocation` (`self.StaticMeshComponent`) (`KismetMathLibrary.VLerp` (`SceneComponent.RelativeLocation` (`self.Start`)) (`SceneComponent.RelativeLocation` (`self.End`)) _raise) false false))))

(event `self.Win.OnComponentBeginOverlap`
  (params (OverlappedComponent :type "PrimitiveComponent Object Reference") (OtherActor :type "Actor Object Reference") (OtherComp :type "PrimitiveComponent Object Reference") (OtherBodyIndex :type Integer) (bFromSweep :type Boolean) (SweepResult :type "HitResult Structure (by ref)"))
  (bind _asbp_top_down_character (cast `/Game/TopDown/Blueprints/BP_TopDownCharacter` OtherActor))
  (`/Engine/EditorBlueprintResources/StandardMacros.CompareInt` (`/Game/TopDown/Blueprints/BP_TopDownCharacter.MapCount` _asbp_top_down_character) 9
    (:`>`
      _)
    (:`==`
      _))
  (bind _returnvalue (`|CreateWidget` "/Game/Blueprints/WinWidget.WinWidget_C"))
  (`UserWidget.AddToViewport` _returnvalue 0)
  (set `PlayerController.bShowMouseCursor` true (`GameplayStatics.GetPlayerController` 0))
  (`GameplayStatics.SetGamePaused` true)
  (`self.K2_DestroyActor`))

(fn `UserConstructionScript`)